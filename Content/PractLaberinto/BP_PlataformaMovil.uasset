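; Moving platform actor for the PractLaberinto folder, built to shuttle Plat0 between marker components P1 and P2.
; BeginPlay snaps Plat0 to P1's relative location.
; The TL_Mov timeline lerps the position between both points, and on finish waits briefly before a FlipFlop alternates reverse and forward playback.
; No graph node starts the timeline, and an IsReturning toggle and interpolation nodes are left unconnected.
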(event EventBeginPlay
  (Transformation|SetRelativeLocation (Variables|Default|GetPlat_0) (Variables|/Script/Engine.SceneComponent|GetRelativeLocation (Variables|Default|GetP1)) false false))

(fn ConstructionScript)